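; Test game mode for actor communication that tracks a score per team.
; On BeginPlay it creates the UI_Test widget and adds it to the viewport.
; IncrementTeamScore adds one to the team's entry in the TeamScores map, keyed by byte, then fires the ScoreUpdated dispatcher with that team.
; GetTeamScore returns the given team along with its current score.
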(event EventBeginPlay
  (bind _returnvalue (UserInterface|CreateWidget "/Game/ActorCommunication/Base/UI_Test.UI_Test_C"))
  (UserInterface|Viewport|AddtoViewport _returnvalue 0))

(event EventIncrementTeamScore
  (params (TeamByte :type Byte :default 0))
  (bind _teamscores (Variables|Default|GetTeamScores))
  (Utilities|Map|Add _teamscores TeamByte (+ (.Value (Utilities|Map|Find _teamscores TeamByte)) 1))
  (Default|CallScoreUpdated TeamByte))

(fn ConstructionScript)

(fn GetTeamScore
  (params (NewParam :type Byte :default 0))
  (return NewParam (.Value (Utilities|Map|Find (Variables|Default|GetTeamScores) NewParam))))